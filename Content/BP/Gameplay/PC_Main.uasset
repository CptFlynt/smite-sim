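; PC_Main, by its name the main player controller, provides events for creating the Simulator, Controller and Production UI widgets.
; CreateSimulatorWidgets casts the game state to GS_Main, creates WB_Simulator_Main with references to itself and that state, and adds it to the viewport.
; CreateControllerWidget and CreateProductionWidget are stubs that only perform the GS_Main cast.
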(event `CreateSimulatorWidgets`
  (bind _asgs_main (cast `/Game/BP/GameFramework/GS_Main` (`GameplayStatics.GetGameState`)))
  (bind _returnvalue (`|CreateWidget` "/Game/BP/Widgets/MainLayouts/WB_Simulator_Main.WB_Simulator_Main_C" self null self _asgs_main))
  (`UserWidget.AddToViewport` _returnvalue 0))

(event `CreateControllerWidget`
  (cast `/Game/BP/GameFramework/GS_Main` (`GameplayStatics.GetGameState`)))

(event `CreateProductionWidget`
  (cast `/Game/BP/GameFramework/GS_Main` (`GameplayStatics.GetGameState`)))

(fn `UserConstructionScript`)